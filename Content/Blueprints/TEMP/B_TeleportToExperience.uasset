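; Trigger actor that moves the game to another experience when a player-controlled pawn overlaps its Cube.
; The overlap asynchronously loads the primary asset referenced by UserFacingExperienceToLoad and casts it to OTUserFacingExperience.
; That experience creates a request, which OTExperienceSessionSubsystem uses to host a new session.
; An asset-list loading branch is left unconnected and never runs.
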(event OnComponentBeginOverlap(Cube)
  (params (OverlappedComponent :type Primitive%20Component%20Object%20Reference) (OtherActor :type Actor%20Object%20Reference) (OtherComp :type Primitive%20Component%20Object%20Reference) (OtherBodyIndex :type Integer) (bFromSweep :type Boolean) (SweepResult :type Hit%20Result%20Structure%20%28by%20ref%29))
  (bind _aspawn (Utilities|Casting|CastToPawn OtherActor))
  (Utilities|Casting|CastToPlayerController (Pawn|GetController _aspawn))
  (bind _loaded (|AsyncLoadPrimaryAsset (AssetManager|GetPrimaryAssetIdfromObject (Variables|Default|GetUserFacingExperienceToLoad)) (Utilities|Array|MakeArray))
    (:then
      (bind _asotuser_facing_experience (Utilities|Casting|CastToOTUserFacingExperience _loaded))
      (bind _returnvalue (Class|OTUserFacingExperience|CreateRequest _asotuser_facing_experience))
      (Class|OTExperienceSessionSubsystem|HostSession (Subsystems|GetOTExperienceSessionSubsystem) 0 _returnvalue))))

(event EventBeginPlay)

(event Collision|EventActorBeginOverlap
  (params (OtherActor :type Actor%20Object%20Reference)))

(event EventTick
  (params (DeltaSeconds :type Float%20%28single-precision%29)))

(fn ConstructionScript)